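; BP_ennemy is an enemy Blueprint that tracks health and reports lost sight of the player to its AI.
; When its Sphere component ends an overlap, it casts its controller to AIC_Enemy and fires PlayerExitVisionEvent.
; TakeDamage subtracts the melee weapon's damage value from Health, runs IsDead and prints the remaining health.
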(event `self.ReceiveBeginPlay`
  (`parent.ReceiveBeginPlay`))

(event `self.Sphere.OnComponentEndOverlap`
  (params (OverlappedComponent :type "PrimitiveComponent Object Reference") (OtherActor :type "Actor Object Reference") (OtherComp :type "PrimitiveComponent Object Reference") (OtherBodyIndex :type Integer))
  (bind _asaic_enemy (cast `/Game/Blueprints/AIC_Enemy` (`AIBlueprintHelperLibrary.GetAIController` self)))
  (`/Game/Blueprints/AIC_Enemy.PlayerExitVision_Event` _asaic_enemy))

(event `Take Damage`
  (bind _health (`self.Health`))
  (set `self.Health` (- _health (`.Damage_8_238F625041B6E49095AB479C7E9BD809` (break `/Game/System/Structures/Struct_Weapon` (`.WeaponDetails_2_BFCBBA5B462FAE054868C888EBD4AA12` (break `/Game/System/Structures/Struct_MeleeWeapon` (`/Game/Blueprints/MasterItemChilds/EquipmentChilds/WeaponChilds/BP_MeleeWeapon.StructMeleeWeapon` (`self.AsMeleeWeapon`))))))))
  (`self.Is Dead`)
  (`KismetSystemLibrary.PrintString` (`KismetStringLibrary.Conv_DoubleToString` _health)))

(fn `UserConstructionScript`
  (`parent.UserConstructionScript`))