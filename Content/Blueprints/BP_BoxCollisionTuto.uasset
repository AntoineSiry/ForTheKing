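; Tutorial trigger volume that changes on-screen tutorial text when something enters its box.
; On BeginPlay it creates its own tutorial widget, adds it to the viewport and keeps a reference.
; Box overlap plays the widget's fade-out animation, waits briefly, sets the text from the actor's TextTuto variable, then fades it back in.
; The overlap does not filter which actor entered.
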(event `self.ReceiveBeginPlay`
  (bind _returnvalue (`|CreateWidget` "/Game/Widget/WBP_Tuto.WBP_Tuto_C"))
  (`UserWidget.AddToViewport` _returnvalue 0)
  (set `self.WidgetREF` _returnvalue))

(event `self.Box.OnComponentBeginOverlap`
  (params (OverlappedComponent :type "PrimitiveComponent Object Reference") (OtherActor :type "Actor Object Reference") (OtherComp :type "PrimitiveComponent Object Reference") (OtherBodyIndex :type Integer) (bFromSweep :type Boolean) (SweepResult :type "HitResult Structure (by ref)"))
  (bind _widgetref (`self.WidgetREF`))
  (bind _widgetref_2 (`self.WidgetREF`))
  (`UserWidget.PlayAnimation` _widgetref (`/Game/Widget/WBP_Tuto.FadeOutText` _widgetref) 0.0 1 "Forward" 1.0 false)
  (`KismetSystemLibrary.Delay` 1.0)
  (set `/Game/Widget/WBP_Tuto.TutoText` (`self.TextTuto`) _widgetref_2)
  (`UserWidget.PlayAnimation` _widgetref_2 (`/Game/Widget/WBP_Tuto.FadeInText` _widgetref_2) 0.0 1 "Forward" 1.0 false))

(fn `UserConstructionScript`)