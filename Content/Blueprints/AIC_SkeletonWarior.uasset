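; AI controller for the skeleton warrior enemy, which patrols, chases and attacks the player with an axe.
; A timeline timed to walk speed drives movement along an optional spline until PawnSensing spots the player.
; Sighting triggers player lock-on and opens a Tick gate for AIMoveTo, leading to a random single swing or two-montage combo.
; Looping timers yaw the controller toward the player; Tick also handles death cleanup.
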(event `self.ReceiveBeginPlay`
  (bind _splinetofollow (`/Game/Blueprints/BP_Enemy.SplineToFollow` (`self.As BP Skeleton`)))
  (`KismetSystemLibrary.Delay` 0.1)
  (`|ExecutionSequence`
    (:`then_0`
      ;[1 1 1] Skeletonbegin play
      (bind _asbp_skeleton (cast `/Game/Blueprints/BP_Skeleton` (`self.K2_GetPawn`)))
      (set `self.As BP Skeleton` _asbp_skeleton)
      (bind _asbp_player (cast `/Game/Blueprints/BP_PLayer` (`GameplayStatics.GetPlayerCharacter` 0)))
      (set `self.As BP Player` _asbp_player)
      (bind _asbp_axe (cast `/Game/Blueprints/MasterItemChilds/EquipmentChilds/WeaponChilds/MeleeWeaponChilds/BP_Axe` (`ChildActorComponent.ChildActor` (`/Game/Blueprints/BP_Skeleton.EnnemyAxe` (`self.As BP Skeleton`)))))
      (set `self.As BP Axe` _asbp_axe))
    (:`then_1`
      ;[1 1 1] [SPLINE] 1/ Calculer le temps de transition pour que ça soit en raccord avec la max walk speed 2/ ça lance le mouvement
      (`/Engine/EditorBlueprintResources/StandardMacros.IsValid` _splinetofollow
        (:`Is Valid`
          (set `self.Duration` (/ (`SplineComponent.GetSplineLength` (`/Game/Blueprints/BP_Path.SplinePath` _splinetofollow)) (`CharacterMovementComponent.MaxWalkSpeed` (`Character.CharacterMovement` (`self.As BP Skeleton`))))))))
    (:`then_2`
      (`/Engine/EditorBlueprintResources/StandardMacros.IsValid` (`/Game/Blueprints/BP_Enemy.SplineToFollow` (`self.As BP Skeleton`))
        (:`Is Valid`
          (`self.WalkOnPath`))))))

(event `WalkOnPath`
  ;[1 1 1] [Spline] Système pour que l'ennemi aille à un endroit qui suit la spline (se stop quand l'ennemi voit le player)
  (`TimelineComponent.SetPlayRate` (`self.MoveTimeline`) (/ 1.0 (`self.Duration`)))
  (bind (_direction _alpha) (`Timeline|MoveTimeline` :!label _label)
    (:`Update`
      (set `self.Alpha` _alpha)
      (`self.MoveToLocation` (`SplineComponent.GetLocationAtDistanceAlongSpline` (`/Game/Blueprints/BP_Path.SplinePath` (`/Game/Blueprints/BP_Enemy.SplineToFollow` (`self.As BP Skeleton`))) (`KismetMathLibrary.Lerp` 0.0 (`SplineComponent.GetSplineLength` (`/Game/Blueprints/BP_Path.SplinePath` (`/Game/Blueprints/BP_Enemy.SplineToFollow` (`self.As BP Skeleton`)))) (`self.Alpha`)) "World") -1.0 true true false true null))))

(event `OnEnemySeePlayer`
  ;[1 1 1] [Spline] Système pour que l'ennemi aille à un endroit qui suit la spline (se stop quand l'ennemi voit le player)
  (set `self.FollowPath?` false)
  (goto _label :!via `Stop`))

(event `self.ReceiveTick`
  (params (DeltaSeconds :type "Float (single-precision)"))
  (bind _as_bp_axe (`self.As BP Axe`))
  (bind _axecombomontage (`/Game/Blueprints/MasterItemChilds/EquipmentChilds/WeaponChilds/MeleeWeaponChilds/BP_Axe.AxeComboMontage` _as_bp_axe))
  (bind _capsulecomponent (`Character.CapsuleComponent` (`self.As BP Skeleton`)))
  (bind _mesh (`Character.Mesh` (`self.As BP Skeleton`)))
  (bind _childactor (`ChildActorComponent.ChildActor` (`/Game/Blueprints/BP_Skeleton.EnnemyAxe` (`self.As BP Skeleton`))))
  (if (`self.FollowPath?`)
    _
    (elif (`/Game/Blueprints/BP_Character.IsDead?` (`self.As BP Skeleton`))
      ;[1 1 1] Death handler
      (`/Engine/EditorBlueprintResources/StandardMacros.DoOnce` false
        (:`Completed`
          (message `/Game/Blueprints/Lock.LockOn` (`self.As BP Player`) false (`self.As BP Skeleton`))
          (`PrimitiveComponent.SetCollisionEnabled` _capsulecomponent "NoCollision")
          (`PrimitiveComponent.SetCollisionObjectType` _capsulecomponent "ECC_WorldStatic")
          (`KismetSystemLibrary.Delay` 2.0)
          (`PawnSensingComponent.SetSensingUpdatesEnabled` (`self.PawnSensing`) false)
          (`/Game/Blueprints/BP_PLayer.OnenemyDie` (`self.As BP Player`))
          (`self.K2_ClearFocus`)))
      (else
        (`/Engine/EditorBlueprintResources/StandardMacros.Gate` true :!label _label_2
          (:`Exit`
            (`|AIMoveTo` (`self.K2_GetPawn`) (`self.K2_GetActorLocation` (`GameplayStatics.GetPlayerCharacter` 0)) (`GameplayStatics.GetPlayerPawn` 0) 150.0
              (:`OnSuccess`
                (`/Engine/EditorBlueprintResources/StandardMacros.DoOnce` false :!label _label_3
                  (:`Completed`
                    (`self.SetActorEnableCollision` _childactor true)
                    (`KismetSystemLibrary.K2_SetTimerDelegate` (delegate `Locking`) 0.001 true)
                    (`KismetSystemLibrary.Delay` 0.2)
                    (if (>= (`KismetMathLibrary.RandomIntegerInRange` 1 10) 5)
                      (bind _returnvalue (`Character.PlayAnimMontage` (`self.As BP Skeleton`) "/Game/Animations/Ennemy/2HandedSkeleton/Axe_EnnemyAttack.Axe_EnnemyAttack" 1.0 "None"))
                      (`KismetSystemLibrary.Delay` _returnvalue)
                      (`self.SetActorEnableCollision` _childactor false)
                      (goto _label_3 :!via `Reset`)
                      (else
                        (set `self.DoingCombo?` true)
                        (`/Engine/EditorBlueprintResources/StandardMacros.IsValid` _as_bp_axe
                          (:`Is Valid`
                            (`KismetSystemLibrary.K2_SetTimerDelegate` (delegate `Locking`) 0.1 true)
                            (`|PlayMontage` _mesh (`|GetArrayItem` _axecombomontage)
                              (:`OnCompleted`
                                (`KismetSystemLibrary.K2_SetTimerDelegate` (delegate `Locking`) 0.1 true)
                                (`|PlayMontage` _mesh (`|GetArrayItem` _axecombomontage 1)
                                  (:`OnCompleted`
                                    (`KismetSystemLibrary.K2_SetTimerDelegate` (delegate `Locking`) 0.1 true)
                                    (set `self.DoingCombo?` false)
                                    (goto _label_3 :!via `Reset`)))))))))))))))))))

(event `self.PawnSensing.OnSeePawn`
  (params (Pawn :type "Pawn Object Reference"))
  (`self.OnEnemySeePlayer` :!label _label_4)
  (`CharacterMovementComponent.SetMovementMode` (`Character.CharacterMovement` (`self.As BP Skeleton`)) "MOVE_Walking" 0)
  (message `/Game/Blueprints/Lock.LockOn` (`self.As BP Player`) true (`self.As BP Skeleton`))
  (goto _label_2 :!via `Open`))

(event `OnSeePawnHandler`
  (`KismetSystemLibrary.K2_SetTimerDelegate` (delegate `Locking`) 0.001 true)
  (goto _label_4))

(event `PlayerExitVision_Event`
  (`KismetSystemLibrary.K2_ClearTimer` null "Locking")
  (`CharacterMovementComponent.DisableMovement` (`Character.CharacterMovement` (`self.As BP Skeleton`)))
  (message `/Game/Blueprints/Lock.LockOn` (`self.As BP Player`) false (`self.As BP Skeleton`))
  (goto _label_2 :!via `Close`))

(event `Locking`
  (bind (_returnvalue_roll _returnvalue_pitch) (`KismetMathLibrary.BreakRotator` (`self.K2_GetActorRotation`)))
  (bind _as_bp_player (`self.As BP Player`))
  (bind (_returnvalue_roll_2 _returnvalue_pitch_2 _returnvalue_yaw) (`KismetMathLibrary.BreakRotator` (`KismetMathLibrary.FindLookAtRotation` (`self.K2_GetActorLocation`) (`self.K2_GetActorLocation` _as_bp_player))))
  (`/Engine/EditorBlueprintResources/StandardMacros.IsValid` _as_bp_player
    (:`Is Valid`
      (`self.K2_SetActorRotation` (`KismetMathLibrary.MakeRotator` _returnvalue_roll _returnvalue_pitch _returnvalue_yaw)))))

(fn `UserConstructionScript`)