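; BP_Hammer is a melee weapon child Blueprint that damages any BP_Player overlapping its Capsule.
; On BeginPlay it caches the first weapon animation montage from StructMeleeWeapon when the weapon enum matches one specific entry.
; Overlaps call LoseHealthEvent with the struct's damage value, gated by a DoOnce that resets after a short delay.
; The overlap path checks neither attack state nor who wields the hammer.
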(event `self.ReceiveBeginPlay`
  (`parent.ReceiveBeginPlay`)
  (`self.AnimToUse`))

(event `AnimToUse`
  (bind (_weapondetails _animmontage _weapon) (break `/Game/System/Structures/Struct_MeleeWeapon` (`self.StructMeleeWeapon`)))
  (if (`|EnumEquality` _weapon "NewEnumerator3")
    (set `self.HammerAnimMontage` (`.AnimMontage_3_7558C96749CA4A3DF120FA9000070345` (break `/Game/System/Structures/Struct_AnimMontage` (`|GetArrayItem` (`.WeaponAnimations_11_BFCBBA5B462FAE054868C888EBD4AA12` (break `/Game/System/Structures/Struct_MeleeWeaponAnim` _animmontage))))))))

(event `self.Capsule.OnComponentBeginOverlap`
  (params (OverlappedComponent :type "PrimitiveComponent Object Reference") (OtherActor :type "Actor Object Reference") (OtherComp :type "PrimitiveComponent Object Reference") (OtherBodyIndex :type Integer) (bFromSweep :type Boolean) (SweepResult :type "HitResult Structure (by ref)"))
  (bind _asbp_player (cast `/Game/Blueprints/BP_PLayer` OtherActor))
  (`/Engine/EditorBlueprintResources/StandardMacros.DoOnce` false :!label _label
    (:`Completed`
      (`/Game/Blueprints/BP_PLayer.LoseHealth_Event` _asbp_player (`.Damage_8_238F625041B6E49095AB479C7E9BD809` (break `/Game/System/Structures/Struct_Weapon` (`.WeaponDetails_2_BFCBBA5B462FAE054868C888EBD4AA12` (break `/Game/System/Structures/Struct_MeleeWeapon` (`self.StructMeleeWeapon`))))))
      (`KismetSystemLibrary.Delay` 1.0)
      (goto _label :!via `Reset`))))

(fn `UserConstructionScript`
  (`parent.UserConstructionScript`))