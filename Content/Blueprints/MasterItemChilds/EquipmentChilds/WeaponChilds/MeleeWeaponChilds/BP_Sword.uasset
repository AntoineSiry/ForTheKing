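; BP_Sword is a melee weapon actor that damages enemies and can visually fade in and out.
; On BeginPlay it caches combo and heavy combo montages from StructMeleeWeapon and sets the material fully visible.
; Appear and Dissapear run looping timers that step the Appearance parameter with a strong emissive, creating a dynamic material instance each tick.
; Capsule overlap with a BP_Enemy adds a new EnemyWidget to the viewport and calls TakeDamage.
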(event `self.ReceiveBeginPlay`
  (`parent.ReceiveBeginPlay`)
  (`self.AnimToUse`)
  (bind _returnvalue (`PrimitiveComponent.CreateDynamicMaterialInstance` (`self.Weapon`) 0 null "None"))
  (`MaterialInstanceDynamic.SetScalarParameterValue` _returnvalue "Appearance" 1.0))

(event `AnimToUse`
  (bind (_weapondetails _animmontage _weapon) (break `/Game/System/Structures/Struct_MeleeWeapon` (`self.StructMeleeWeapon`)))
  (bind _weaponanimations (break `/Game/System/Structures/Struct_MeleeWeaponAnim` _animmontage))
  (bind _returnvalue (`|EnumEquality` _weapon "NewEnumerator0"))
  (`|ExecutionSequence`
    (:`then_0`
      (if _returnvalue
        (set `self.SwordComboMontage` (`.AnimMontage_3_7558C96749CA4A3DF120FA9000070345` (break `/Game/System/Structures/Struct_AnimMontage` (`|GetArrayItem` _weaponanimations))))))
    (:`then_1`
      (if _returnvalue
        (set `self.SwordHeavyComboMontage` (`.AnimMontage_3_7558C96749CA4A3DF120FA9000070345` (break `/Game/System/Structures/Struct_AnimMontage` (`|GetArrayItem` _weaponanimations 1))))))))

(event `Appear`
  (`KismetSystemLibrary.K2_SetTimer` null "WeaponAppearance" 0.09 true))

(event `Dissapear`
  (`KismetSystemLibrary.K2_SetTimer` null "WeaponDissapear" 0.09 true))

(event `self.Capsule.OnComponentBeginOverlap`
  (params (OverlappedComponent :type "PrimitiveComponent Object Reference") (OtherActor :type "Actor Object Reference") (OtherComp :type "PrimitiveComponent Object Reference") (OtherBodyIndex :type Integer) (bFromSweep :type Boolean) (SweepResult :type "HitResult Structure (by ref)"))
  (bind _asbp_enemy (cast `/Game/Blueprints/BP_Enemy` OtherActor))
  (set `self.EnnemyREF` _asbp_enemy)
  (bind _returnvalue (`|CreateWidget` "/Game/Widget/EnemyWidget.EnemyWidget_C"))
  (`UserWidget.AddToViewport` _returnvalue 0)
  (`/Game/Blueprints/BP_Enemy.Take Damage` (`self.EnnemyREF`)))

(fn `UserConstructionScript`
  (`parent.UserConstructionScript`))

(fn `WeaponAppearance`
  (bind _returnvalue (+ (`self.Appearance`) 0.1))
  (bind _returnvalue_2 (`PrimitiveComponent.CreateDynamicMaterialInstance` (`self.Weapon`) 0 null "None"))
  (`MaterialInstanceDynamic.SetScalarParameterValue` _returnvalue_2 "Appearance" _returnvalue)
  (`MaterialInstanceDynamic.SetScalarParameterValue` _returnvalue_2 "Emmisive_Mult" 10000.0)
  (bind _output_get (set `self.Appearance` _returnvalue))
  (if (>= _output_get 1.0)
    (`KismetSystemLibrary.K2_ClearTimer` null "WeaponAppearance")))

(fn `WeaponDissapear`
  (bind _returnvalue (- (`self.Appearance`) 0.1))
  (bind _returnvalue_2 (`PrimitiveComponent.CreateDynamicMaterialInstance` (`self.Weapon`) 0 "/Game/Materials/M_Swords_Inst.M_Swords_Inst" "None"))
  (`MaterialInstanceDynamic.SetScalarParameterValue` _returnvalue_2 "Appearance" _returnvalue)
  (`MaterialInstanceDynamic.SetScalarParameterValue` _returnvalue_2 "Emmisive_Mult" 10000.0)
  (bind _output_get (set `self.Appearance` _returnvalue))
  (if (<= _output_get 0.0)
    (`KismetSystemLibrary.K2_ClearTimer` null "WeaponDissapear")))