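; BP_Axe is the axe child of the melee weapon Blueprint hierarchy, setting up the combo montage for that weapon.
; After the parent BeginPlay, it calls AnimToUse, which checks the weapon enum in StructMeleeWeapon.
; On a match, it stores the first montage from the struct's weapon animations in AxeComboMontage.
; The construction script only calls its parent, and the Tick and overlap events are disabled.
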(event `self.ReceiveBeginPlay`
  (`parent.ReceiveBeginPlay`)
  (`self.AnimToUse`))

(event `AnimToUse`
  (bind (_weapondetails _animmontage _weapon) (break `/Game/System/Structures/Struct_MeleeWeapon` (`self.StructMeleeWeapon`)))
  (if (`|EnumEquality` _weapon "NewEnumerator2")
    (set `self.AxeComboMontage` (`.AnimMontage_3_7558C96749CA4A3DF120FA9000070345` (break `/Game/System/Structures/Struct_AnimMontage` (`|GetArrayItem` (`.WeaponAnimations_11_BFCBBA5B462FAE054868C888EBD4AA12` (break `/Game/System/Structures/Struct_MeleeWeaponAnim` _animmontage))))))))

(fn `UserConstructionScript`
  (`parent.UserConstructionScript`))