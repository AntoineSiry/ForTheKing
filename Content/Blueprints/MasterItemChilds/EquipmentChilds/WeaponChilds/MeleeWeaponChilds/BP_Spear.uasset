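; BP_Spear is a spear melee weapon Blueprint that prepares its combo montages when play begins.
; After the parent BeginPlay, AnimToUse checks the weapon type in StructMeleeWeapon and, on a match, copies the first weapon animation entry's montages into SpearComboMontage.
; It then prints the first montage's name on screen as debug output.
; The file holds no attack or combo playback logic, and its Tick and overlap events are disabled.
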(event `self.ReceiveBeginPlay`
  (`parent.ReceiveBeginPlay`)
  (`self.AnimToUse`))

(event `AnimToUse`
  (bind (_weapondetails _animmontage _weapon) (break `/Game/System/Structures/Struct_MeleeWeapon` (`self.StructMeleeWeapon`)))
  (if (`|EnumEquality` _weapon "NewEnumerator1")
    (bind _output_get (set `self.SpearComboMontage` (`.AnimMontage_3_7558C96749CA4A3DF120FA9000070345` (break `/Game/System/Structures/Struct_AnimMontage` (`|GetArrayItem` (`.WeaponAnimations_11_BFCBBA5B462FAE054868C888EBD4AA12` (break `/Game/System/Structures/Struct_MeleeWeaponAnim` _animmontage)))))))
    (`KismetSystemLibrary.PrintString` (`KismetSystemLibrary.GetDisplayName` (`|GetArrayItem` _output_get)) true true (struct :`G` 0.66 :`B` 1.0 :`A` 1.0) 100.0)))

(fn `UserConstructionScript`
  (`parent.UserConstructionScript`))