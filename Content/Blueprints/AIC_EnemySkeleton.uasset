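; AI controller for the skeleton enemy that chases the player and attacks with its axe.
; Seeing a pawn enables player lock-on and opens a Tick gate for AIMoveTo; the vision-exit event reverses both and halts movement.
; On arrival, a looping timer updates yaw toward the player and a random roll picks a single swing or chained two-montage combo.
; Death disables capsule collision and sensing, then releases lock-on.
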(event `self.ReceiveBeginPlay`
  (bind _asbp_skeleton (cast `/Game/Blueprints/BP_Skeleton` (`self.K2_GetPawn`)))
  (set `self.As BP Skeleton` _asbp_skeleton)
  (bind _asbp_player (cast `/Game/Blueprints/BP_PLayer` (`GameplayStatics.GetPlayerCharacter` 0)))
  (set `self.As BP Player` _asbp_player)
  (bind _asbp_axe (cast `/Game/Blueprints/MasterItemChilds/EquipmentChilds/WeaponChilds/MeleeWeaponChilds/BP_Axe` (`ChildActorComponent.ChildActor` (`/Game/Blueprints/BP_Skeleton.EnnemyAxe` (`self.As BP Skeleton`)))))
  (set `self.As BP Axe` _asbp_axe))

(event `self.ReceiveTick`
  (params (DeltaSeconds :type "Float (single-precision)"))
  (bind _as_bp_axe (`self.As BP Axe`))
  (bind _axecombomontage (`/Game/Blueprints/MasterItemChilds/EquipmentChilds/WeaponChilds/MeleeWeaponChilds/BP_Axe.AxeComboMontage` _as_bp_axe))
  (bind _mesh (`Character.Mesh` (`self.As BP Skeleton`)))
  (bind _childactor (`ChildActorComponent.ChildActor` (`/Game/Blueprints/BP_Skeleton.EnnemyAxe` (`self.As BP Skeleton`))))
  (if (`/Game/Blueprints/BP_Character.IsDead?` (`self.As BP Skeleton`))
    (`PrimitiveComponent.SetCollisionEnabled` (`Character.CapsuleComponent` (`self.As BP Skeleton`)) "NoCollision")
    (`AIPerceptionComponent.SetSenseEnabled` (`self.AIPerception`) "/Script/AIModule.AISense_Sight" false)
    (`PawnSensingComponent.SetSensingUpdatesEnabled` (`self.PawnSensing`) false)
    (`/Engine/EditorBlueprintResources/StandardMacros.DoOnce` false
      (:`Completed`
        (message `/Game/Blueprints/Lock.LockOn` (`self.As BP Player`) false (`self.As BP Skeleton`))))
    (else
      (`/Engine/EditorBlueprintResources/StandardMacros.Gate` true :!label _label
        (:`Exit`
          (`|AIMoveTo` (`self.K2_GetPawn`) (`self.K2_GetActorLocation` (`GameplayStatics.GetPlayerCharacter` 0)) (`GameplayStatics.GetPlayerPawn` 0) 150.0
            (:`OnSuccess`
              (`/Engine/EditorBlueprintResources/StandardMacros.DoOnce` false :!label _label_2
                (:`Completed`
                  (`self.SetActorEnableCollision` _childactor true)
                  (`KismetSystemLibrary.K2_SetTimerDelegate` (delegate `Locking`) 0.001 true)
                  (`KismetSystemLibrary.Delay` 0.2)
                  (if (>= (`KismetMathLibrary.RandomIntegerInRange` 1 10) 4)
                    (bind _returnvalue (`Character.PlayAnimMontage` (`self.As BP Skeleton`) "/Game/Animations/Ennemy/2HandedSkeleton/Axe_EnnemyAttack.Axe_EnnemyAttack" 1.0 "None"))
                    (`KismetSystemLibrary.Delay` _returnvalue)
                    (`self.SetActorEnableCollision` _childactor false)
                    (goto _label_2 :!via `Reset`)
                    (else
                      (`KismetSystemLibrary.PrintString` "combo")
                      (`/Engine/EditorBlueprintResources/StandardMacros.IsValid` _as_bp_axe
                        (:`Is Valid`
                          (`|PlayMontage` _mesh (`|GetArrayItem` _axecombomontage)
                            (:`OnCompleted`
                              (`|PlayMontage` _mesh (`|GetArrayItem` _axecombomontage 1)
                                (:`OnCompleted`
                                  (goto _label_2 :!via `Reset`))))))))))))))))))

(event `self.PawnSensing.OnSeePawn`
  (params (Pawn :type "Pawn Object Reference"))
  (`CharacterMovementComponent.SetMovementMode` (`Character.CharacterMovement` (`self.As BP Skeleton`)) "MOVE_Walking" 0)
  (message `/Game/Blueprints/Lock.LockOn` (`self.As BP Player`) true (`self.As BP Skeleton`))
  (goto _label :!via `Open`))

(event `PlayerExitVision_Event`
  (`KismetSystemLibrary.K2_ClearTimer` null "Locking")
  (`CharacterMovementComponent.DisableMovement` (`Character.CharacterMovement` (`self.As BP Skeleton`)))
  (message `/Game/Blueprints/Lock.LockOn` (`self.As BP Player`) false (`self.As BP Skeleton`))
  (goto _label :!via `Close`))

(event `Locking`
  (bind _as_bp_player (`self.As BP Player`))
  (bind (_returnvalue_roll _returnvalue_pitch) (`KismetMathLibrary.BreakRotator` (`self.K2_GetActorRotation` (`self.As BP Skeleton`))))
  (bind (_returnvalue_roll_2 _returnvalue_pitch_2 _returnvalue_yaw) (`KismetMathLibrary.BreakRotator` (`KismetMathLibrary.FindLookAtRotation` (`self.K2_GetActorLocation` (`self.As BP Skeleton`)) (`self.K2_GetActorLocation` _as_bp_player))))
  (`/Engine/EditorBlueprintResources/StandardMacros.IsValid` _as_bp_player
    (:`Is Valid`
      (`self.K2_SetActorRotation` (`KismetMathLibrary.MakeRotator` _returnvalue_roll _returnvalue_pitch _returnvalue_yaw)))))

(fn `UserConstructionScript`)