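; Base spear weapon actor that damages characters it hits and can fade in and out of view.
; Capsule overlaps call CallTakeDamage on any BP_Character, with events to switch capsule collision on and off.
; BeginPlay hides the spear through its material and applies the StaticMesh variable.
; Appear and Dissapear run looping timers that step the material's Appearance parameter, creating a new dynamic material instance each tick.
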(event `self.Capsule.OnComponentBeginOverlap`
  (params (OverlappedComponent :type "PrimitiveComponent Object Reference") (OtherActor :type "Actor Object Reference") (OtherComp :type "PrimitiveComponent Object Reference") (OtherBodyIndex :type Integer) (bFromSweep :type Boolean) (SweepResult :type "HitResult Structure (by ref)"))
  (bind _asbp_character (cast `/Game/Blueprints/BP_Character` OtherActor))
  (`/Game/Blueprints/BP_Character.TakeDamage` _asbp_character))

(event `self.Capsule.OnComponentEndOverlap`
  (params (OverlappedComponent :type "PrimitiveComponent Object Reference") (OtherActor :type "Actor Object Reference") (OtherComp :type "PrimitiveComponent Object Reference") (OtherBodyIndex :type Integer)))

(event `EnableSpearCollision`
  (`PrimitiveComponent.SetCollisionEnabled` (`self.Capsule`) "QueryAndPhysics"))

(event `DisableSpearCollision`
  (`PrimitiveComponent.SetCollisionEnabled` (`self.Capsule`) "NoCollision"))

(event `self.ReceiveBeginPlay`
  (bind _returnvalue (`PrimitiveComponent.CreateDynamicMaterialInstance` (`self.Spear`) 0 "/Game/Materials/M_Polearm_Inst.M_Polearm_Inst" "None"))
  (`MaterialInstanceDynamic.SetScalarParameterValue` _returnvalue "Appearance" 0.0)
  (`StaticMeshComponent.SetStaticMesh` (`self.Spear`) (`self.StaticMesh`)))

(event `Appear`
  (`KismetSystemLibrary.K2_SetTimer` null "WeaponAppearance" 0.09 true))

(event `Dissapear`
  (`KismetSystemLibrary.K2_SetTimer` null "WeaponDissapear" 0.09 true))

(fn `UserConstructionScript`)

(fn `WeaponAppearance`
  (bind _returnvalue (+ (`self.Appearance`) 0.1))
  (bind _returnvalue_2 (`PrimitiveComponent.CreateDynamicMaterialInstance` (`self.Spear`) 0 "/Game/Materials/M_Polearm_Inst.M_Polearm_Inst" "None"))
  (`MaterialInstanceDynamic.SetScalarParameterValue` _returnvalue_2 "Appearance" _returnvalue)
  (`MaterialInstanceDynamic.SetScalarParameterValue` _returnvalue_2 "Emissive_Mult" 1.0)
  (bind _output_get (set `self.Appearance` _returnvalue))
  (if (>= _output_get 1.0)
    (`KismetSystemLibrary.K2_ClearTimer` null "WeaponAppearance")))

(fn `WeaponDissapear`
  (bind _returnvalue (- (`self.Appearance`) 0.1))
  (bind _returnvalue_2 (`PrimitiveComponent.CreateDynamicMaterialInstance` (`self.Spear`) 0 "/Game/Materials/M_Polearm_Inst.M_Polearm_Inst" "None"))
  (`MaterialInstanceDynamic.SetScalarParameterValue` _returnvalue_2 "Appearance" _returnvalue)
  (`MaterialInstanceDynamic.SetScalarParameterValue` _returnvalue_2 "Emissive_Mult" 1.0)
  (bind _output_get (set `self.Appearance` _returnvalue))
  (if (<= _output_get 0.0)
    (`KismetSystemLibrary.K2_ClearTimer` null "WeaponDissapear")))