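; BP_Character is a character Blueprint that handles health and death.
; On BeginPlay it stores the BP_MeleeWeapon found in the level through GetActorOfClass.
; ChangeHealthPoint adds a signed delta to Health, calls CheckIfDead and returns the new value.
; CheckIfDead sets IsDead and, at zero health or below, stops movement immediately and plays the Death montage through a DoOnce gate.
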(event `self.ReceiveBeginPlay`
  ;[1 1 1] Begin Play
  (bind _returnvalue (`GameplayStatics.GetActorOfClass` "/Game/Blueprints/MasterItemChilds/EquipmentChilds/WeaponChilds/BP_MeleeWeapon.BP_MeleeWeapon_C"))
  (set `self.AsMeleeWeapon` _returnvalue))

(event `CheckIfDead`
  ;[1 1 1] Check if the character doesn't have health
  (if (<= (`self.Health`) 0.0)
    (set `self.IsDead?` true)
    (`MovementComponent.StopMovementImmediately` (`self.CharacterMovement`))
    (`/Engine/EditorBlueprintResources/StandardMacros.DoOnce` false
      (:`Completed`
        (`self.PlayAnimMontage` "/Game/Animations/Player/Death/Death.Death")))
    (else
      (set `self.IsDead?` false))))

(fn `ChangeHealthPoint`
  (params (UpdateHealth :type "Float (double-precision)"))
  (returns (NewHealth :type "Float (double-precision)"))
  ;[1 1 1] Update Health of Character
  (bind _output_get (set `self.Health` (+ UpdateHealth (`self.Health`))))
  (`self.CheckIfDead`)
  (return _output_get))

(fn `UserConstructionScript`)