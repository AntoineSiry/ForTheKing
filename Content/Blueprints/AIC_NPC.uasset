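; AI controller that makes its possessed NPC walk along the spline assigned to it.
; After a short delay on BeginPlay, it caches the NPC and derives the path duration from spline length and max walk speed.
; A timeline, with play rate set from that duration, lerps distance along the spline and issues MoveToLocation to that moving point on every update.
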(event `self.ReceiveBeginPlay`
  (bind _as_npc (`self.As NPC`))
  (bind _splinetofollow (`/Game/Blueprints/BP_Enemy.SplineToFollow` _as_npc))
  (`KismetSystemLibrary.Delay` 0.2)
  (`|ExecutionSequence`
    (:`then_0`
      (bind _asnpc (cast `/Game/Blueprints/NPC` (`self.K2_GetPawn`)))
      (set `self.As NPC` _asnpc))
    (:`then_1`
      ;[1 1 1] [SPLINE] 1/ Calculer le temps de transition pour que ça soit en raccord avec la max walk speed 2/ ça lance le mouvement
      (`/Engine/EditorBlueprintResources/StandardMacros.IsValid` _splinetofollow
        (:`Is Valid`
          (set `self.Duration` (/ (`SplineComponent.GetSplineLength` (`/Game/Blueprints/BP_Path.SplinePath` _splinetofollow)) (`CharacterMovementComponent.MaxWalkSpeed` (`Character.CharacterMovement` _as_npc)))))))
    (:`then_2`
      (`/Engine/EditorBlueprintResources/StandardMacros.IsValid` (`/Game/Blueprints/BP_Enemy.SplineToFollow` (`self.As NPC`))
        (:`Is Valid`
          (`self.WalkOnPath`))))))

(event `WalkOnPath`
  (bind _as_npc (`self.As NPC`))
  ;[1 1 1] [Spline] Système pour que l'ennemi aille à un endroit qui suit la spline (se stop quand l'ennemi voit le player)
  (`TimelineComponent.SetPlayRate` (`self.MoveTimeline`) (/ 1.0 (`self.Duration`)))
  (bind (_direction _alpha) (`Timeline|MoveTimeline`)
    (:`Update`
      (set `self.Alpha` _alpha)
      (`self.MoveToLocation` (`SplineComponent.GetLocationAtDistanceAlongSpline` (`/Game/Blueprints/BP_Path.SplinePath` (`/Game/Blueprints/BP_Enemy.SplineToFollow` _as_npc)) (`KismetMathLibrary.Lerp` 0.0 (`SplineComponent.GetSplineLength` (`/Game/Blueprints/BP_Path.SplinePath` (`/Game/Blueprints/BP_Enemy.SplineToFollow` _as_npc))) (`self.Alpha`)) "World") -1.0 true true false true null))))

(fn `UserConstructionScript`)