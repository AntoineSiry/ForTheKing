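; Bow weapon actor that fades its skeletal mesh in and out through a material appearance effect.
; Appear and Dissapear start looping timers that step the Appearance value up or down until it reaches its limit, then clear themselves; it begins play by dissolving away.
; Each tick of those timers creates a new dynamic material instance from M_Bows_Inst, setting Appearance and a very high emissive multiplier.
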(event `self.ReceiveBeginPlay`
  (`self.Dissapear`))

(event `Appear`
  (`KismetSystemLibrary.K2_SetTimer` null "WeaponAppearance" 0.03 true))

(event `Dissapear`
  (`KismetSystemLibrary.K2_SetTimer` null "WeaponDissapear" 0.09 true))

(fn `UserConstructionScript`)

(fn `WeaponAppearance`
  (bind _returnvalue (+ (`self.Appearance`) 0.1))
  (bind _returnvalue_2 (`PrimitiveComponent.CreateDynamicMaterialInstance` (`self.SkeletalMesh`) 0 "/Game/Materials/M_Bows_Inst.M_Bows_Inst" "None"))
  (`MaterialInstanceDynamic.SetScalarParameterValue` _returnvalue_2 "Appearance" _returnvalue)
  (`MaterialInstanceDynamic.SetScalarParameterValue` _returnvalue_2 "Emmisive_Mult" 10000.0)
  (bind _output_get (set `self.Appearance` _returnvalue))
  (if (>= _output_get 1.0)
    (`KismetSystemLibrary.K2_ClearTimer` null "WeaponAppearance")))

(fn `WeaponDissapear`
  (bind _returnvalue (- (`self.Appearance`) 0.1))
  (bind _returnvalue_2 (`PrimitiveComponent.CreateDynamicMaterialInstance` (`self.SkeletalMesh`) 0 "/Game/Materials/M_Bows_Inst.M_Bows_Inst" "None"))
  (`MaterialInstanceDynamic.SetScalarParameterValue` _returnvalue_2 "Appearance" _returnvalue)
  (`MaterialInstanceDynamic.SetScalarParameterValue` _returnvalue_2 "Emmisive_Mult" 10000.0)
  (bind _output_get (set `self.Appearance` _returnvalue))
  (if (<= _output_get 0.0)
    (`KismetSystemLibrary.K2_ClearTimer` null "WeaponDissapear")))