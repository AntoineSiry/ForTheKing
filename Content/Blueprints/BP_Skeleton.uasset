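; Skeleton warrior enemy that wields an axe child actor, can dodge hits, and grants the player experience on death.
; Capsule overlaps register it with the enemy collision manager, show impact and widget, then roll damage against a 20% block (commented as 30%), with dodge montages outside combos.
; Separate events toggle axe collision.
; Death fires a dispatcher for experience and optional win screen, then destroys the actor after a delay.
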(event `self.ReceiveBeginPlay`
  (`parent.ReceiveBeginPlay`)
  (bind _asbp_axe (cast `/Game/Blueprints/MasterItemChilds/EquipmentChilds/WeaponChilds/MeleeWeaponChilds/BP_Axe` (`ChildActorComponent.ChildActor` (`self.EnnemyAxe`))))
  (set `self.As BP Axe` _asbp_axe)
  (bind _returnvalue (`GameplayStatics.GetActorOfClass` "/Game/Blueprints/BP_EnnemyCollisionManager.BP_EnnemyCollisionManager_C"))
  (set `self.EnnemyColManager` _returnvalue)
  (set `self.Name` (`self.EnemyName`))
  (add `self.TakeDamage` (delegate `DeathIA`))
  (bind _asaic_skeleton_warior (cast `/Game/Blueprints/AIC_SkeletonWarior` (`AIBlueprintHelperLibrary.GetAIController` self)))
  (set `self.As AIC Skeleton Warior` _asaic_skeleton_warior)
  (bind _asbp_player (cast `/Game/Blueprints/BP_PLayer` (`GameplayStatics.GetPlayerCharacter` 0)))
  (set `self.As BP Player_` _asbp_player))

(event `DeathIA`
  (`/Game/Blueprints/BP_PLayer.AddExp` (`self.As BP Player_`) (`self.ExpToAdd`))
  (if (`self.CanWin?`)
    (bind _returnvalue (`|CreateWidget` "/Game/Widget/WBP_Win.WBP_Win_C"))
    (`UserWidget.AddToViewport` _returnvalue 0)))

(event `EnableAxeCollision`
  (`PrimitiveComponent.SetCollisionEnabled` (`/Game/Blueprints/MasterItemChilds/EquipmentChilds/WeaponChilds/MeleeWeaponChilds/BP_Axe.Capsule` (`self.As BP Axe`)) "QueryAndPhysics"))

(event `DisableAxeCollision`
  (`PrimitiveComponent.SetCollisionEnabled` (`/Game/Blueprints/MasterItemChilds/EquipmentChilds/WeaponChilds/MeleeWeaponChilds/BP_Axe.Capsule` (`self.As BP Axe`)) "NoCollision"))

(event `self.CapsuleComponent.OnComponentBeginOverlap`
  (params (OverlappedComponent :type "PrimitiveComponent Object Reference") (OtherActor :type "Actor Object Reference") (OtherComp :type "PrimitiveComponent Object Reference") (OtherBodyIndex :type Integer) (bFromSweep :type Boolean) (SweepResult :type "HitResult Structure (by ref)"))
  (set `/Game/Blueprints/BP_EnnemyCollisionManager.EnnemyTouched` self (`self.EnnemyColManager`))
  (`GameplayStatics.SpawnEmitterAtLocation` "/Game/AdvancedMagicFX13/Particles/P_ky_impact.P_ky_impact" (`self.K2_GetActorLocation`))
  (bind _returnvalue (`|CreateWidget` "/Game/Widget/EnemyWidget.EnemyWidget_C"))
  (`UserWidget.AddToViewport` _returnvalue 0)
  (`self.Take Damage`)
  (if (`self.IsDead?`)
    (`self.SetActorEnableCollision` (`ChildActorComponent.ChildActor` (`self.EnnemyAxe`)) false)))

(event `Take Damage`
  (bind _mesh (`self.Mesh`))
  (`self.CheckIfDead`)
  (if (`self.IsDead?`)
    (set `self.IsDead?` true)
    (`self.CheckIfDead`)
    (else
      ;[1 1 1] Block system (30% chances to doge)
      (if (>= (`KismetMathLibrary.RandomIntegerInRange` 1 10) 3)
        (`self.LoseHealth`)
        (elif (`/Game/Blueprints/AIC_SkeletonWarior.DoingCombo?` (`self.As AIC Skeleton Warior`))
          _
          (elif (`KismetMathLibrary.RandomBool`)
            (`|PlayMontage` _mesh "/Game/Animations/Ennemy/2HandedSkeleton/Axe_EnnemyDodgeLeft.Axe_EnnemyDodgeLeft")
            (else
              (`|PlayMontage` _mesh "/Game/Animations/Ennemy/2HandedSkeleton/Axe_EnnemyDodgeRight.Axe_EnnemyDodgeRight"))))))))

(event `CheckIfSkelettonDead`
  (if (<= (`self.Health`) 0.0)
    (set `self.IsDead?` true)
    (`MovementComponent.StopMovementImmediately` (`self.CharacterMovement`))
    (`PrimitiveComponent.SetCollisionEnabled` (`self.CapsuleComponent`) "NoCollision")
    (`self.TakeDamage`)
    (`KismetSystemLibrary.Delay` 100.0)
    (`self.K2_DestroyActor`)
    (else
      (set `self.IsDead?` false))))

(fn `UserConstructionScript`
  (`parent.UserConstructionScript`))