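; BP_MagicAmmo is a magic projectile actor driven by a ProjectileMovement component.
; On BeginPlay it applies its Velocity variable to that component and caches the BP_Player character.
; SpawnProjectile spawns another BP_MagicAmmo, aiming from the player's SpawnPoint toward a distant point along Camera1's forward vector.
; The scaled aim vector serves as both the new actor's velocity and its spawn location, rather than SpawnPoint's position.
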(event `SpawnProjectile`
  (bind _refthirdpersoncharacter (`self.RefThirdPersonCharacter`))
  (bind _camera1 (`/Game/Blueprints/BP_PLayer.Camera1` _refthirdpersoncharacter))
  (bind _returnvalue (* (`KismetMathLibrary.Normal` (- (+ (`SceneComponent.K2_GetComponentLocation` _camera1) (* (`SceneComponent.GetForwardVector` _camera1) 8000.0)) (`SceneComponent.K2_GetComponentLocation` (`/Game/Blueprints/BP_PLayer.SpawnPoint` _refthirdpersoncharacter)))) 8000.0))
  (`|SpawnActorFromClass` "BP_MagicAmmo_C" (`KismetMathLibrary.MakeTransform` _returnvalue) "Undefined" "OverrideRootScale" null _returnvalue null))

(event `self.ReceiveBeginPlay`
  (set `MovementComponent.Velocity` (`self.Velocity`) (`self.ProjectileMovement`))
  (bind _asbp_player (cast `/Game/Blueprints/BP_PLayer` (`GameplayStatics.GetPlayerCharacter` 0)))
  (set `self.RefThirdPersonCharacter` _asbp_player))

(fn `UserConstructionScript`)