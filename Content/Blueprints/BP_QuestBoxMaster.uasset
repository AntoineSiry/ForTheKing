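; BP_QuestBoxMaster is a trigger box that shows quest text when the player enters it.
; The box's begin-overlap event checks for player character 0 and runs through a DoOnce, so it fires a single time.
; It removes existing top-level WBP_Quest widgets, then creates a new one, flags it as already displayed and passes it TextQuest.
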(event `self.Box.OnComponentBeginOverlap`
  (params (OverlappedComponent :type "PrimitiveComponent Object Reference") (OtherActor :type "Actor Object Reference") (OtherComp :type "PrimitiveComponent Object Reference") (OtherBodyIndex :type Integer) (bFromSweep :type Boolean) (SweepResult :type "HitResult Structure (by ref)"))
  (if (== OtherActor (`GameplayStatics.GetPlayerCharacter` 0))
    (`/Engine/EditorBlueprintResources/StandardMacros.DoOnce` false
      (:`Completed`
        (bind _foundwidgets (`WidgetBlueprintLibrary.GetAllWidgetsOfClass` "/Game/Widget/WBP_Quest.WBP_Quest_C"))
        (for _array_element _foundwidgets
          (`Widget.RemoveFromParent` _array_element))
        (bind _returnvalue (`|CreateWidget` "/Game/Widget/WBP_Quest.WBP_Quest_C"))
        (`UserWidget.AddToViewport` _returnvalue 0)
        (set `/Game/Widget/WBP_Quest.IsAlreadyDisplayed` true _returnvalue)
        (`/Game/Widget/WBP_Quest.SetText` _returnvalue (`self.TextQuest`))))))

(fn `UserConstructionScript`)