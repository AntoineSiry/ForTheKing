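; AI controller for BP_Enemy, a melee enemy that patrols, chases and attacks the player.
; It walks along an optional spline via a timeline scaled to walk speed until PawnSensing spots the player.
; Tick then drives a gated AIMoveTo, followed on arrival by a random light attack or montage combo whose notifies toggle foot and shield collision.
; It also updates player lock-on, halts on vision loss and handles death cleanup.
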(event `self.ReceiveBeginPlay`
  (bind _ref_enemy (`self.Ref Enemy`))
  (bind _splinetofollow (`/Game/Blueprints/BP_Enemy.SplineToFollow` _ref_enemy))
  (`KismetSystemLibrary.Delay` 0.2)
  (`|ExecutionSequence`
    (:`then_0`
      (bind _asbp_enemy (cast `/Game/Blueprints/BP_Enemy` (`self.K2_GetPawn`)))
      (set `self.Ref Enemy` _asbp_enemy)
      (bind _asbp_player (cast `/Game/Blueprints/BP_PLayer` (`GameplayStatics.GetPlayerCharacter` 0)))
      (set `self.As BP Player` _asbp_player)
      (bind _asbp_sword (cast `/Game/Blueprints/MasterItemChilds/EquipmentChilds/WeaponChilds/MeleeWeaponChilds/BP_Sword` (`ChildActorComponent.ChildActor` (`/Game/Blueprints/BP_Enemy.Sword` (`self.Ref Enemy`)))))
      (set `self.As BP Sword` _asbp_sword))
    (:`then_1`
      ;[1 1 1] [SPLINE] 1/ Calculer le temps de transition pour que ça soit en raccord avec la max walk speed 2/ ça lance le mouvement
      (`/Engine/EditorBlueprintResources/StandardMacros.IsValid` _splinetofollow
        (:`Is Valid`
          (set `self.Duration` (/ (`SplineComponent.GetSplineLength` (`/Game/Blueprints/BP_Path.SplinePath` _splinetofollow)) (`CharacterMovementComponent.MaxWalkSpeed` (`Character.CharacterMovement` _ref_enemy)))))))
    (:`then_2`
      (`/Engine/EditorBlueprintResources/StandardMacros.IsValid` (`/Game/Blueprints/BP_Enemy.SplineToFollow` (`self.Ref Enemy`))
        (:`Is Valid`
          (`self.WalkOnPath`))))))

(event `WalkOnPath`
  (bind _ref_enemy (`self.Ref Enemy`))
  ;[1 1 1] [Spline] Système pour que l'ennemi aille à un endroit qui suit la spline (se stop quand l'ennemi voit le player)
  (`TimelineComponent.SetPlayRate` (`self.MoveTimeline`) (/ 1.0 (`self.Duration`)))
  (bind (_direction _alpha) (`Timeline|MoveTimeline` :!label _label)
    (:`Update`
      (set `self.Alpha` _alpha)
      (`self.MoveToLocation` (`SplineComponent.GetLocationAtDistanceAlongSpline` (`/Game/Blueprints/BP_Path.SplinePath` (`/Game/Blueprints/BP_Enemy.SplineToFollow` _ref_enemy)) (`KismetMathLibrary.Lerp` 0.0 (`SplineComponent.GetSplineLength` (`/Game/Blueprints/BP_Path.SplinePath` (`/Game/Blueprints/BP_Enemy.SplineToFollow` _ref_enemy))) (`self.Alpha`)) "World") -1.0 true true false true null))))

(event `OnEnemySeePlayer`
  ;[1 1 1] [Spline] Système pour que l'ennemi aille à un endroit qui suit la spline (se stop quand l'ennemi voit le player)
  (set `self.FollowPath?` false)
  (goto _label :!via `Stop`))

(event `self.ReceiveTick`
  (params (DeltaSeconds :type "Float (single-precision)"))
  (bind _ref_enemy (`self.Ref Enemy`))
  (bind _shieldcollision (`/Game/Blueprints/BP_Enemy.ShieldCollision` (`self.Ref Enemy`)))
  (bind _collisionfoot (`/Game/Blueprints/BP_Enemy.CollisionFoot` (`self.Ref Enemy`)))
  (bind _capsulecomponent (`Character.CapsuleComponent` (`self.Ref Enemy`)))
  (bind _childactor (`ChildActorComponent.ChildActor` (`/Game/Blueprints/BP_Enemy.Sword` (`self.Ref Enemy`))))
  (if (not (`self.FollowPath?`))
    (`/Engine/EditorBlueprintResources/StandardMacros.IsValid` _ref_enemy
      (:`Is Valid`
        (if (`/Game/Blueprints/BP_Character.IsDead?` _ref_enemy)
          ;[1 1 1] Death handler
          (`/Engine/EditorBlueprintResources/StandardMacros.DoOnce` false
            (:`Completed`
              (message `/Game/Blueprints/Lock.LockOn` (`self.As BP Player`) false (`self.Ref Enemy`))
              (`PrimitiveComponent.SetCollisionEnabled` _capsulecomponent "NoCollision")
              (`PrimitiveComponent.SetCollisionObjectType` _capsulecomponent "ECC_WorldStatic")
              (`KismetSystemLibrary.Delay` 2.0)
              (`PawnSensingComponent.SetSensingUpdatesEnabled` (`self.PawnSensing`) false)
              (`/Game/Blueprints/BP_PLayer.OnenemyDie` (`self.As BP Player`))
              (`self.K2_ClearFocus`)))
          (else
            (`/Engine/EditorBlueprintResources/StandardMacros.Gate` true :!label _label_2
              (:`Exit`
                (`|AIMoveTo` (`self.K2_GetPawn`) (`self.K2_GetActorLocation` (`GameplayStatics.GetPlayerCharacter` 0)) (`GameplayStatics.GetPlayerPawn` 0) 150.0
                  (:`OnSuccess`
                    (`/Engine/EditorBlueprintResources/StandardMacros.DoOnce` false :!label _label_3
                      (:`Completed`
                        (`self.SetActorEnableCollision` _childactor true)
                        (`KismetSystemLibrary.Delay` 0.2)
                        (if (>= (`KismetMathLibrary.RandomIntegerInRange` 1 10) 3)
                          (bind _returnvalue (`Character.PlayAnimMontage` (`self.Ref Enemy`) "/Game/Animations/Player/WarriorSwordRM/Sword_LightAttack.Sword_LightAttack" 1.0 "None"))
                          (`KismetSystemLibrary.Delay` _returnvalue)
                          (`self.SetActorEnableCollision` _childactor false)
                          (goto _label_3 :!via `Reset`)
                          (else
                            (set `self.DoingCombo?` true)
                            ;[1 1 1] Combo system
                            (`/Engine/EditorBlueprintResources/StandardMacros.IsValid` (`self.As BP Sword`)
                              (:`Is Valid`
                                (bind _notifyname (`|PlayMontage` (`Character.Mesh` (`self.Ref Enemy`)) (`|GetArrayItem` (`/Game/Blueprints/MasterItemChilds/EquipmentChilds/WeaponChilds/MeleeWeaponChilds/BP_Sword.SwordComboMontage` (`self.As BP Sword`)) (`self.ComboAnimIndex`)) :!label _label_4)
                                  (:`OnCompleted`
                                    (if (< (`self.ComboAnimIndex`) 2)
                                      (bind _result (`/Engine/EditorBlueprintResources/StandardMacros.IncrementInt` (`self.ComboAnimIndex`))
                                        (:`  `
                                          (set `self.ComboAnimIndex` _result)
                                          (goto _label_4)))
                                      (else
                                        (set `self.ComboAnimIndex` 0)
                                        (set `self.DoingCombo?` false)
                                        (goto _label_3 :!via `Reset`))))
                                  (:`OnNotifyBegin`
                                    (set `self.Notify Name Anim` _notifyname)
                                    (switch `int` (`self.ComboAnimIndex`)
                                      (:`0`
                                        (switch `name` (`self.Notify Name Anim`)
                                          (:`ShieldCollisisonF`
                                            (`PrimitiveComponent.SetCollisionEnabled` _collisionfoot "NoCollision"))
                                          (:`ShieldCollisionT`
                                            (`PrimitiveComponent.SetCollisionEnabled` _collisionfoot "QueryAndPhysics"))))
                                      (:`2`
                                        (switch `name` (`self.Notify Name Anim`)
                                          (:`ShieldCollisisonF`
                                            (`PrimitiveComponent.SetCollisionEnabled` _shieldcollision "NoCollision"))
                                          (:`ShieldCollisionT`
                                            (`PrimitiveComponent.SetCollisionEnabled` _shieldcollision "QueryAndPhysics")))))))))))))))))))))))

(event `self.PawnSensing.OnSeePawn`
  (params (Pawn :type "Pawn Object Reference"))
  (set `CharacterMovementComponent.MaxWalkSpeed` 600.0 (`Character.CharacterMovement` (`self.Ref Enemy`)))
  (set `self.SawPlayer?` true)
  (`self.OnEnemySeePlayer` :!label _label_5)
  (`CharacterMovementComponent.SetMovementMode` (`Character.CharacterMovement` (`self.Ref Enemy`)) "MOVE_Walking" 0)
  (if (`/Game/Blueprints/BP_PLayer.LockedOn` (`self.As BP Player`))
    (goto _label_2 :!via `Open`)
    (else
      (message `/Game/Blueprints/Lock.LockOn` (`self.As BP Player`) true (`self.Ref Enemy`))
      (goto _label_2 :!via `Open`))))

(event `OnSeePawnHandler`
  (`self.K2_SetFocus` (`self.As BP Player`))
  (goto _label_5))

(event `PlayerExitVision_Event`
  (`CharacterMovementComponent.DisableMovement` (`Character.CharacterMovement` (`self.Ref Enemy`)))
  (message `/Game/Blueprints/Lock.LockOn` (`self.As BP Player`) false (`self.Ref Enemy`))
  (goto _label_2 :!via `Close`))

(fn `UserConstructionScript`)