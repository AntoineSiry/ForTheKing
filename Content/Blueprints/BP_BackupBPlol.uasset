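; BP_BackupBPlol appears to be a backup Blueprint holding a disconnected enemy sword-combo graph that never runs.
; The graph chains three montages from the sword's combo array on RefEnemy's mesh, each starting when the previous completes.
; Shield-named montage notifies toggle foot collision during the first montage and shield collision during the third, with numbered debug prints.
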(fn `UserConstructionScript`)